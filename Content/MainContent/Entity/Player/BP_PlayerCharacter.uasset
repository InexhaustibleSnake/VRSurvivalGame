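; BP_PlayerCharacter is the VR player character, fitting its collision capsule to the headset's height.
; BeginPlay sets the tracking origin to eye level when a head-mounted display is enabled.
; UpdateCharacterHeight, not called within this graph, sets capsule half-height to half the HMD's Z position plus padding.
; It then shifts VRCameraPointComponent vertically by that target minus the capsule half-height, read after the resize.
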(event `self.ReceiveBeginPlay`
  (if (`HeadMountedDisplayFunctionLibrary.IsHeadMountedDisplayEnabled`)
    (`HeadMountedDisplayFunctionLibrary.SetTrackingOrigin` "Eye")))

(event `UpdateCharacterHeight`
  (bind _returnvalue (+ (/ (.z (`.DevicePosition` (`HeadMountedDisplayFunctionLibrary.GetOrientationAndPosition`))) 2.0) 10.0))
  (`CapsuleComponent.SetCapsuleSize` (`self.CapsuleComponent`) (`CapsuleComponent.GetScaledCapsuleRadius` (`self.CapsuleComponent`)) _returnvalue true)
  (`SceneComponent.K2_AddRelativeLocation` (`self.VRCameraPointComponent`) (`KismetMathLibrary.MakeVector` 0.0 0.0 (- _returnvalue (`CapsuleComponent.CapsuleHalfHeight` (`self.CapsuleComponent`)))) false false))

(fn `UserConstructionScript`)